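; GM_RobbinArrow is the game mode, providing helper functions for player respawn, deer respawn and screen fades.
; RespawnPlayer teleports the first player's pawn to every PlayerStart in turn, so it ends at the last one found.
; RespawnDeer spawns a BP_Deer at each transform stored in DeerTransformArray.
; The two fade functions create W_FadeOut or W_FadeIn widgets on the viewport and play them at a given speed.
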(fn `Fading IN`
  (params (PlaybackSpeed :type "Float (single-precision)"))
  (bind _returnvalue (`|CreateWidget` "/Game/Player/Widgets/W_FadeIn.W_FadeIn_C"))
  (`UserWidget.AddToViewport` _returnvalue 0)
  (`/Game/Player/Widgets/W_FadeIn.PlayFadeIn` _returnvalue PlaybackSpeed))

(fn `Fading Out`
  (params (PlaybackSpeed :type "Float (single-precision)"))
  (bind _returnvalue (`|CreateWidget` "/Game/Player/Widgets/W_FadeOut.W_FadeOut_C"))
  (`UserWidget.AddToViewport` _returnvalue 0)
  (`/Game/Player/Widgets/W_FadeOut.PlayFadeOut` _returnvalue PlaybackSpeed))

(fn `RespawnDeer`
  (for _array_element (`self.DeerTransformArray`)
    (`|SpawnActorFromClass` "/Game/Player/AI/Deer/BP_Deer.BP_Deer_C" _array_element "Undefined" "MultiplyWithRoot" null null)))

(fn `RespawnPlayer`
  (bind _outactors (`GameplayStatics.GetAllActorsOfClass` "/Script/Engine.PlayerStart"))
  (for _array_element _outactors
    (`self.K2_SetActorLocation` (`GameplayStatics.GetPlayerPawn` 0) (`self.K2_GetActorLocation` _array_element) false true)))

(fn `UserConstructionScript`
  (`parent.UserConstructionScript`))