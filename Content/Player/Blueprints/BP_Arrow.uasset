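; Archery arrow projectile that flies, scores its shot and drives the replay camera.
; Player zoom sets speed and gravity, and overlapping a wind controller steers horizontal velocity.
; Hits bounce off the Kraken or stick elsewhere, with targets scored by a line trace's distance from center.
; Hits, or misses after three seconds, show the camera replay and score widget; hits add to stage score and the third arrow ends the game.
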(event `self.ReceiveTick`
  (params (DeltaSeconds :type "Float (single-precision)"))
  (bind (_returnvalue_x _returnvalue_y _returnvalue_z) (`KismetMathLibrary.BreakVector` (`self.GetVelocity`)))
  (bind (_returnvalue_x_2 _returnvalue_y_2) (`KismetMathLibrary.BreakVector` (`KismetMathLibrary.VLerp` (`self.InitialVelocuty`) (`self.WindTargetVelocity`) (* DeltaSeconds 30.0))))
  (if (not (`self.HitSomething`))
    (set `MovementComponent.Velocity` (`KismetMathLibrary.MakeVector` _returnvalue_x_2 _returnvalue_y_2 _returnvalue_z) (`self.ProjectileMovement`))))

(event `self.ReceiveBeginPlay`
  (bind _projectilemovement (`self.ProjectileMovement`))
  (bind _asbp_player (cast `/Game/Player/Blueprints/BP_Player` (`GameplayStatics.GetPlayerPawn` 0)))
  (bind _zoom_alpha (`/Game/Player/Blueprints/BP_Player.Zoom Alpha` _asbp_player))
  (set `self.Zoom Alpha` _zoom_alpha)
  (bind _output_get (set `MovementComponent.Velocity` (* (`self.GetVelocity`) (`KismetMathLibrary.Lerp` 1.0 2.0 _zoom_alpha)) _projectilemovement))
  (bind _output_get_2 (set `self.InitialVelocuty` _output_get))
  (set `self.WindTargetVelocity` _output_get_2)
  (set `ProjectileMovementComponent.ProjectileGravityScale` (`KismetMathLibrary.Lerp` (`self.MaxGravity`) 0.05 _zoom_alpha) _projectilemovement)
  (`NiagaraFunctionLibrary.SpawnSystemAttached` "/Game/Player/Arrow/NS_ArrowTrail.NS_ArrowTrail" (`self.TrailEffectLocation`) "None" (0.0 0.0 0.0) (struct) "KeepRelativeOffset")
  (`GameplayStatics.PlaySoundAtLocation` "/Game/Player/Arrow/Sound/Cue_Arrow_Whoosh.Cue_Arrow_Whoosh" (`self.K2_GetActorLocation`) (struct) 1.0 1.0 0.0 null null null null)
  (bind _returnvalue (`|CreateWidget` "/Game/Player/Widgets/W_ShotScore.W_ShotScore_C"))
  (set `self.ShotScoreWidgetRef` _returnvalue)
  (`KismetSystemLibrary.Delay` 3.0)
  (if (not (`self.HitSomething`))
    (bind _asbp_player_2 (cast `/Game/Player/Blueprints/BP_Player` (`GameplayStatics.GetPlayerPawn` 0)))
    (set `/Game/Player/Blueprints/BP_Player.IsReplaying` true _asbp_player_2)
    (`/Game/Player/Blueprints/BP_Player.ZoomCameraEnd` _asbp_player_2)
    (`WidgetLayoutLibrary.RemoveAllWidgets`)
    (`PlayerController.SetViewTargetWithBlend` (`GameplayStatics.GetPlayerController` 0) self 0.3 "VTBlend_Linear" 0.0 false)
    (`UserWidget.AddToViewport` (`self.ShotScoreWidgetRef`) 0)
    (`KismetSystemLibrary.Delay` 1.5)
    (bind _asbp_player_3 (cast `/Game/Player/Blueprints/BP_Player` (`GameplayStatics.GetPlayerPawn` 0)))
    (set `/Game/Player/Blueprints/BP_Player.IsReplaying` false _asbp_player_3)
    (`Widget.RemoveFromParent` (`self.ShotScoreWidgetRef`))
    (`PlayerController.SetViewTargetWithBlend` (`GameplayStatics.GetPlayerController` 0) (`GameplayStatics.GetPlayerPawn` 0) 0.5 "VTBlend_Linear" 0.0 false)
    (bind _returnvalue_2 (`|CreateWidget` "/Game/Player/Widgets/W_PlayerHud_01.W_PlayerHud_01_C"))
    (`UserWidget.AddToViewport` _returnvalue_2 0)
    (`self.K2_DestroyActor`)))

(event `self.HitBox.OnComponentBeginOverlap`
  (params (OverlappedComponent :type "PrimitiveComponent Object Reference") (OtherActor :type "Actor Object Reference") (OtherComp :type "PrimitiveComponent Object Reference") (OtherBodyIndex :type Integer) (bFromSweep :type Boolean) (SweepResult :type "HitResult Structure (by ref)"))
  (bind (_returnvalue_x _returnvalue_y _returnvalue_z) (`KismetMathLibrary.BreakVector` (`self.GetVelocity`)))
  (bind _projectilemovement (`self.ProjectileMovement`))
  (set `self.HitActor` OtherActor)
  (bind _asbp_wind_controller (cast `/Game/Player/Blueprints/BP_WindController` OtherActor)
    (:`then`
      (bind _windrotation (`/Game/Player/Blueprints/BP_WindController.WindRotation` _asbp_wind_controller))
      (bind _output_get (set `self.WindDirection` (`KismetMathLibrary.MakeVector` (* (`KismetMathLibrary.DegCos` _windrotation) 0.3) (`KismetMathLibrary.DegSin` _windrotation))))
      (bind _output_get_2 (set `self.WindForce` (* _output_get 300.0)))
      (set `self.WindTargetVelocity` (+ _output_get_2 (`self.InitialVelocuty`))))
    (:`CastFailed`
      (if (and (!= OtherActor self) (!= OtherActor (`GameplayStatics.GetPlayerPawn` 0)))
        (`|ExecutionSequence`
          (:`then_0`
            (cast `/Game/Player/AI/Kraken/BP_Kraken` (`self.HitActor`)
              (:`then`
                (set `self.HitSomething` true)
                (set `MovementComponent.Velocity` (`KismetMathLibrary.MakeVector` (+ _returnvalue_x (`KismetArrayLibrary.Array_Random` (`|MakeArray` (* 600.0 -0.7) (* 600.0 1.0) (* 600.0 0.5)))) (* _returnvalue_y -0.5) (+ 400.0 _returnvalue_z)) (`self.ProjectileMovement`)))
              (:`CastFailed`
                (`GameplayStatics.PlaySoundAtLocation` "/Game/Player/Arrow/Sound/arrow_hit_01_Cue.arrow_hit_01_Cue" (`self.K2_GetActorLocation`) (struct) 1.0 1.0 0.0 null null null null)
                (`MovementComponent.StopMovementImmediately` _projectilemovement)
                (set `ProjectileMovementComponent.ProjectileGravityScale` 0.0 _projectilemovement)
                (`PrimitiveComponent.SetCollisionEnabled` (`self.HitBox`) "NoCollision")
                (`self.K2_AttachToActor` OtherActor "None" "KeepWorld" "KeepWorld" "KeepWorld")))
            (`|ExecutionSequence`
              (:`then_0`
                (bind _asbp_target (cast `/Game/Player/Blueprints/BP_Target` OtherActor) ; 과녁에 명중
                  (:`then`
                    (bind _outhit (`KismetSystemLibrary.LineTraceSingle` (`SceneComponent.K2_GetComponentLocation` (`self.End`)) (`SceneComponent.K2_GetComponentLocation` (`self.Start`)) "TraceTypeQuery3" false (`|MakeArray` null :!type "Actor Object Reference") "None" true (struct :`R` 1.0 :`A` 1.0) (struct :`G` 1.0 :`A` 1.0) 10.0)) ; 화살 끝에서 머리로 트레이스로 충돌지점 파악
                    (`|ExecutionSequence`
                      (:`then_0`
                        ;[1 1 1] 화살이 박히는 정도를 고정
                        (`SceneComponent.K2_SetRelativeLocation` (`self.Arrow`) (`KismetMathLibrary.MakeVector` (- (`.Distance` (`GameplayStatics.BreakHitResult` _outhit)) (`KismetMathLibrary.RandomFloatInRange` 25.0 50.0))) false true))
                      (:`then_1`
                        (bind _returnvalue (`KismetMathLibrary.FCeil` (- 10.0 (* (/ (`KismetMathLibrary.Vector_Distance` (`.Location` (`GameplayStatics.BreakHitResult` _outhit)) (`/Game/Player/Blueprints/BP_Target.TargetCenterLocation` _asbp_target)) (`/Game/Player/Blueprints/BP_Target.TargetCircleRadius` _asbp_target)) 10.0))))
                        (if (> _returnvalue 0)
                          (set `self.ShotScore` _returnvalue)
                          (else
                            (set `self.ShotScore` 0)))
                        (set `/Game/Player/Widgets/W_ShotScore.ShotScore` (`self.ShotScore`) (`self.ShotScoreWidgetRef`) :!label _label))))
                  (:`CastFailed`
                    (set `self.ShotScore` 0)
                    (goto _label))))
              (:`then_1`
                (bind _asbp_player (cast `/Game/Player/Blueprints/BP_Player` (`GameplayStatics.GetPlayerPawn` 0)))
                (set `/Game/Player/Blueprints/BP_Player.IsReplaying` true _asbp_player)
                (`/Game/Player/Blueprints/BP_Player.ZoomCameraEnd` _asbp_player)
                (`KismetSystemLibrary.Delay` 1.0)
                (bind _asbp_deer (cast `/Game/Player/AI/Deer/BP_Deer` (`self.HitActor`))
                  (:`then`
                    (`PlayerController.SetViewTargetWithBlend` (`GameplayStatics.GetPlayerController` 0) _asbp_deer 0.0 "VTBlend_Linear" 0.0 false))
                  (:`CastFailed`
                    (`PlayerController.SetViewTargetWithBlend` (`GameplayStatics.GetPlayerController` 0) self 0.5 "VTBlend_Linear" 0.0 false)))
                (bind _foundwidgets (`WidgetBlueprintLibrary.GetAllWidgetsOfClass` "/Game/Player/Widgets/W_PlayerHud_01.W_PlayerHud_01_C"))
                (for _array_element _foundwidgets
                  (`Widget.RemoveFromParent` _array_element))
                (`UserWidget.AddToViewport` (`self.ShotScoreWidgetRef`) 0)
                (`KismetSystemLibrary.Delay` 1.5)
                (`PlayerController.SetViewTargetWithBlend` (`GameplayStatics.GetPlayerController` 0) (`GameplayStatics.GetPlayerPawn` 0) 0.5 "VTBlend_Linear" 0.0 false)
                (`KismetSystemLibrary.Delay` 0.2)
                (set `/Game/Player/Blueprints/BP_Player.IsReplaying` false _asbp_player)
                (`KismetSystemLibrary.PrintString` (`KismetStringLibrary.Concat_StrStr` "발사 점수: " (`KismetStringLibrary.Conv_IntToString` (`self.ShotScore`))) true true (struct :`G` 0.66 :`B` 1.0 :`A` 1.0) 10.0)
                (bind _asbp_player_2 (cast `/Game/Player/Blueprints/BP_Player` (`GameplayStatics.GetPlayerCharacter` 0)))
                (bind _output_get_3 (set `/Game/Player/Blueprints/BP_Player.StageScore` (+ (`/Game/Player/Blueprints/BP_Player.StageScore` _asbp_player_2) (`self.ShotScore`)) _asbp_player_2))
                (`KismetSystemLibrary.PrintString` (`KismetStringLibrary.Concat_StrStr` "누적 점수: " (`KismetStringLibrary.Conv_IntToString` _output_get_3)) true true (struct :`R` 0.467136 :`B` 1.0 :`A` 1.0) 10.0)
                (`Widget.RemoveFromParent` (`self.ShotScoreWidgetRef`))
                (if (== (`self.ArrowNumber`) 3)
                  (`KismetSystemLibrary.Delay` 0.5)
                  (bind _asbp_player_3 (cast `/Game/Player/Blueprints/BP_Player` (`GameplayStatics.GetPlayerPawn` 0)))
                  (`/Game/Player/Blueprints/BP_Player.EndRealGame` _asbp_player_3)
                  (else
                    (bind _returnvalue_2 (`|CreateWidget` "/Game/Player/Widgets/W_PlayerHud_01.W_PlayerHud_01_C"))
                    (`UserWidget.AddToViewport` _returnvalue_2 0))))))
          (:`then_1`
            (set `self.HitSomething` true)
            (bind _asbp_player_4 (cast `/Game/Player/Blueprints/BP_Player` (`GameplayStatics.GetPlayerPawn` 0)))
            (`/Game/Player/Blueprints/BP_Player.ArrowHit` _asbp_player_4)))))))

(event `DestroyArrow`
  (`self.K2_DestroyActor`))

(fn `UserConstructionScript`)