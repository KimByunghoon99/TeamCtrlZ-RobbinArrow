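; Player character for a staged archery game, handling bow aiming, firing, arrow-view replay, pause menu and HUD.
; Zoom runs a timeline driving FOV, boom offset and draw-sound pitch under slow motion; firing traces from the camera to orient an arrow spawned at the bow socket.
; Enter switches practice to the counted game, resetting arrows and respawning player and deer through the GameMode.
; Game end checks score, saves cleared-stage progress to the GameInstance and pauses.
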(event `self.ReceiveBeginPlay`
  (set `CharacterMovementComponent.JumpZVelocity` 0.0 (`self.CharacterMovement`))
  (`Controller.SetIgnoreMoveInput` (`self.GetController`) true)
  (set `self.IsReplaying` true)
  (bind _returnvalue (`GameplayStatics.GetCurrentLevelName` true))
  (set `self.CurrentStageName` _returnvalue)
  (set `self.CurrentStageNumber` (`KismetStringLibrary.Conv_StringToInt` _returnvalue))
  (set `self.Initial FOV` (`CameraComponent.FieldOfView` (`self.FollowCamera`)))
  (set `self.InitialBoomOffset` (`SpringArmComponent.SocketOffset` (`self.CameraBoom`)))
  (`CameraComponent.SetFieldOfView` (`self.FollowCamera`) 80.0)
  (set `SpringArmComponent.SocketOffset` (0.0 50.0 60.0) (`self.CameraBoom`))
  (set `self.StageScore` 0)
  (set `self.ShotStack` 0)
  (`|PlayMontage` (`self.Mesh`) "/Game/Player/Animations/AM_LevelStart.AM_LevelStart" 1.3
    (:`OnCompleted`
      (set `CharacterMovementComponent.JumpZVelocity` 900.0 (`self.CharacterMovement`))
      (`Controller.SetIgnoreMoveInput` (`self.GetController`) false)
      (set `self.IsReplaying` false)
      (`CameraComponent.SetFieldOfView` (`self.FollowCamera`) (`self.Initial FOV`))
      (set `SpringArmComponent.SocketOffset` (`self.InitialBoomOffset`) (`self.CameraBoom`))
      (bind _returnvalue_2 (`|CreateWidget` "/Game/Player/Widgets/W_PlayerHud_01.W_PlayerHud_01_C"))
      (bind _output_get (set `self.PlayerHUD` _returnvalue_2))
      (`UserWidget.AddToViewport` _output_get 0)
      (bind _returnvalue_3 (`|CreateWidget` "/Game/Player/Widgets/W_PracticeMode.W_PracticeMode_C"))
      (bind _output_get_2 (set `self.PracticeModeWidget` _returnvalue_3))
      (`UserWidget.AddToViewport` _output_get_2 0))))

(event `EnhancedInput|/Game/Player/Input/IA_ZoomInOut`
  (params (ActionValue :type Boolean) (ElapsedSeconds :type "Float (double-precision)") (TriggeredSeconds :type "Float (double-precision)") (InputAction :type "InputAction Object Reference" :default "/Game/Player/Input/IA_ZoomInOut.IA_ZoomInOut"))
  (:`Started`
    (`self.ZoomCameraBegin`))
  (:`Completed`
    (`self.ZoomCameraEnd`)))

(event `ZoomCameraBegin`
  (bind _initial_fov (`self.Initial FOV`))
  (bind _initialboomoffset (`self.InitialBoomOffset`))
  (if (`self.CanFire`)
    (if (not (`self.IsReplaying`))
      (set `self.IsZoomON` true)
      (bind _returnvalue (`GameplayStatics.SpawnSoundAtLocation` "/Game/Player/Arrow/Sound/Cue_Arrow_Draw.Cue_Arrow_Draw" (`self.K2_GetActorLocation`) (struct) 1.0 1.0 0.0 null null))
      (set `self.DrawSoundRef` _returnvalue)
      (`GameplayStatics.SetGlobalTimeDilation` 0.35)
      (bind (_direction _zoomalpha _zoomtime) (`Timeline|ZoomCameraTimeline` :`NewTime` 100.0 :!via `PlayFromStart` :!label _label)
        (:`Update`
          (set `self.Zoom Alpha` _zoomalpha)
          (set `self.Zoom Time` _zoomtime)
          (`CameraComponent.SetFieldOfView` (`self.FollowCamera`) (`KismetMathLibrary.Lerp` _initial_fov (`self.Zoom FOV`) _zoomalpha))
          (set `SpringArmComponent.SocketOffset` (`KismetMathLibrary.VLerp` _initialboomoffset (`self.ZoomBoomOffset`) _zoomalpha) (`self.CameraBoom`))
          (`self.CallOnZoomOngoing` (`self.Zoom Time`) 100.0))
        (:`Finished`
          (set `self.Zoom Alpha` 0.0)
          (set `self.Zoom Time` 0.0)
          (`CameraComponent.SetFieldOfView` (`self.FollowCamera`) _initial_fov)
          (set `SpringArmComponent.SocketOffset` _initialboomoffset (`self.CameraBoom`))
          (set `self.IsZoomON` false)
          (`GameplayStatics.SetGlobalTimeDilation` 1.0)
          (`self.CallOnZoomOngoing` (`self.Zoom Time`) 100.0))))))

(event `self.ReceiveTick`
  (params (DeltaSeconds :type "Float (single-precision)"))
  (bind _returnvalue (/ (`self.Zoom Alpha`) 1.0))
  (bind _drawsoundref (`self.DrawSoundRef`)
    (:`then`
      (`AudioComponent.SetPitchMultiplier` _drawsoundref (`KismetMathLibrary.Lerp` 1.5 0.75 _returnvalue))
      (`AudioComponent.SetVolumeMultiplier` _drawsoundref (`KismetMathLibrary.Lerp` 1.4 0.9 _returnvalue)))
    (:`else`)))

(event `ZoomCameraEnd`
  (if (`self.IsZoomON`)
    (bind _drawsoundref (`self.DrawSoundRef`)
      (:`then`
        (`AudioComponent.Stop` _drawsoundref)
        (goto _label :!via `SetNewTime`))
      (:`else`
        (goto _label :!via `SetNewTime`)))))

(event `Key|LeftControl`
  (params (Key :type "Key Structure"))
  (:`Pressed`
    (set `SpringArmComponent.SocketOffset` (-100.0 0.0 80.0) (`self.CameraBoom`)))
  (:`Released`
    (set `SpringArmComponent.SocketOffset` (`self.InitialBoomOffset`) (`self.CameraBoom`))))

(event `InputAction|Fire`
  (params (Key :type "Key Structure"))
  (bind _returnvalue (`GameplayStatics.GetPlayerCameraManager` 0))
  (bind _returnvalue_2 (`self.K2_GetActorLocation` _returnvalue))
  (bind _returnvalue_3 (- (`self.ImpactPoint`) (`self.ArrowSpawnLocation`)))
  (:`Pressed`
    (if (`self.CanFire`)
      (if (not (`self.IsReplaying`))
        (set `self.CanFire` false)
        (`|ExecutionSequence`
          (:`then_0`
            ;[1 1 1] 라인트레이스 시작 위치
            (set `self.CrosshairWorldLocation` _returnvalue_2)
            ;[1 1 1] 라인트레이스 도착 위치
            (set `self.ImpactPoint` (+ _returnvalue_2 (* (`self.GetActorForwardVector` _returnvalue) (15000.0 15000.0 15000.0)))))
          (:`then_1`
            (bind _outhit (`KismetSystemLibrary.LineTraceSingle` (`self.CrosshairWorldLocation`) (`self.ImpactPoint`) "TraceTypeQuery1" false (`|MakeArray` self :!type "Actor Object Reference")))
            (bind (_bblockinghit _binitialoverlap _time _distance _location _impactpoint) (`GameplayStatics.BreakHitResult` _outhit))
            (if _bblockinghit
              (set `self.ImpactPoint` _impactpoint) ; 라인트레이스가 물체와 충돌하면 그지점이 임팩트 포인트
            )
            (set `self.ArrowSpawnLocation` (.location (`SceneComponent.GetSocketTransform` (`self.Mesh`) "BowEmitterSocket" "RTS_World"))) ; 충돌하지 않으면 카메라로부터 15000유닛 먼곳이 임팩트 포인트
            (set `self.ArrowDirection` _returnvalue_3)
            (set `self.ArrowSpawnRotation` (`KismetMathLibrary.MakeRotFromX` _returnvalue_3)))
          (:`then_2`
            (bind _returnvalue_4 (`|SpawnActorFromClass` "/Game/Player/Blueprints/BP_Arrow.BP_Arrow_C" (`KismetMathLibrary.MakeTransform` (`self.ArrowSpawnLocation`) (`self.ArrowSpawnRotation`)) "AdjustIfPossibleButAlwaysSpawn" "MultiplyWithRoot" self self))
            (bind _output_get (set `self.ArrowRef` _returnvalue_4))
            (if (`self.IsRealGameON`)
              (`|ExecutionSequence`
                (:`then_0`
                  (set `self.ShotStack` (+ (`self.ShotStack`) 1))
                  (`KismetSystemLibrary.PrintString` (`KismetStringLibrary.Concat_StrStr` "발사 횟수: " (`KismetStringLibrary.Conv_IntToString` (`self.ShotStack`)))))
                (:`then_1`
                  (set `/Game/Player/Blueprints/BP_Arrow.ArrowNumber` (`self.ShotStack`) _output_get)))
              (else
                (`self.SetLifeSpan` _output_get 10.0))))
          (:`then_3`
            (`|PlayMontage` (`self.Mesh`) "/Game/Player/Animations/AM_Fire.AM_Fire" 0.6))
          (:`then_4`
            (`self.ZoomCameraEnd`)))))))

(event `Key|Tab`
  (params (Key :type "Key Structure"))
  ;[1 1 1] 지난 화살 꽂힌 곳 확인
  (:`Pressed`
    (`/Engine/EditorBlueprintResources/StandardMacros.IsValid` (`self.ArrowRef`)
      (:`Is Valid`
        (if (not (not (`self.IsZoomON`)))
          (`self.ZoomCameraEnd`))
        (`GameplayStatics.SetGlobalTimeDilation` 0.2)
        (`PlayerController.SetViewTargetWithBlend` (`GameplayStatics.GetPlayerController` 0) (`self.ArrowRef`) 0.01 "VTBlend_Linear" 0.0 false)
        (`WidgetLayoutLibrary.RemoveAllWidgets`)
        (set `self.IsReplaying` true))))
  (:`Released`
    (`GameplayStatics.SetGlobalTimeDilation` 1.0)
    (`PlayerController.SetViewTargetWithBlend` (`GameplayStatics.GetPlayerController` 0) (`GameplayStatics.GetPlayerPawn` 0) 0.3 "VTBlend_Linear" 0.0 false)
    (bind _returnvalue (`|CreateWidget` "/Game/Player/Widgets/W_PlayerHud_01.W_PlayerHud_01_C"))
    (`UserWidget.AddToViewport` _returnvalue 0)
    (set `self.IsReplaying` false)))

(event `Key|Enter`
  (params (Key :type "Key Structure"))
  (:`Pressed`
    (if (not (`self.IsRealGameON`))
      (`self.StartRealGame`)
      (bind _asgm_robbin_arrow (cast `/Game/Player/Blueprints/GM_RobbinArrow` (`GameplayStatics.GetGameMode`)))
      (`/Game/Player/Blueprints/GM_RobbinArrow.Fading Out` _asgm_robbin_arrow)
      (`KismetSystemLibrary.Delay` 2.0)
      (`/Game/Player/Blueprints/GM_RobbinArrow.Fading IN` _asgm_robbin_arrow)
      (`/Game/Player/Blueprints/GM_RobbinArrow.RespawnPlayer` _asgm_robbin_arrow)
      (`/Game/Player/Blueprints/GM_RobbinArrow.RespawnDeer` _asgm_robbin_arrow))))

(event `ArrowHit`
  (`self.ChangeWind`))

(event `StartRealGame`
  (bind _playerhud (`self.PlayerHUD`))
  (bind _output_get (set `self.IsRealGameON` true))
  (`/Engine/EditorBlueprintResources/StandardMacros.IsValid` _playerhud
    (:`Is Valid`
      (set `/Game/Player/Widgets/W_PlayerHud_01.RealGameOn` _output_get _playerhud)
      (set `self.ShotStack` 0)
      (set `self.StageScore` 0)
      (bind _outactors (`GameplayStatics.GetAllActorsOfClass` "/Game/Player/Blueprints/BP_Arrow.BP_Arrow_C"))
      (for _array_element _outactors
        (`/Game/Player/Blueprints/BP_Arrow.DestroyArrow` _array_element))
      (`Widget.RemoveFromParent` (`self.PracticeModeWidget`)))))

(event `EndRealGame`
  (set `self.IsRealGameON` false)
  (set `/Game/Player/Widgets/W_PlayerHud_01.RealGameOn` false (`self.PlayerHUD`))
  (set `self.IsGameEnded` true)
  (bind _output_get (set `self.IsStageCleared` (>= (`self.StageScore`) 20)))
  (if _output_get
    (`self.StageCleared`)
    (else
      (`self.StageFailed`)))
  (`self.PauseGame`))

(event `PauseGame`
  (bind _returnvalue (`GameplayStatics.GetPlayerController` 0))
  (set `self.IsPauseMesuOpened` true)
  (bind _returnvalue_2 (`|CreateWidget` "/Game/Player/Widgets/W_PauseMenu.W_PauseMenu_C" _returnvalue))
  (bind _output_get (set `self.PauseMenu` _returnvalue_2))
  (set `/Game/Player/Widgets/W_PauseMenu.IsGameEnd` (`self.IsGameEnded`) _output_get)
  (set `/Game/Player/Widgets/W_PauseMenu.CurrentStage` (`self.CurrentStageName`) (`self.PauseMenu`))
  (set `/Game/Player/Widgets/W_PauseMenu.IsGameCleared` (`self.IsStageCleared`) (`self.PauseMenu`))
  (`UserWidget.AddToViewport` _returnvalue_2 0)
  (`UserWidget.AddToViewport` (`self.PauseMenu`) 0)
  (`WidgetBlueprintLibrary.SetInputMode_GameAndUIEx` _returnvalue (`self.PauseMenu`))
  (set `PlayerController.bShowMouseCursor` true (`GameplayStatics.GetPlayerController` 0))
  (`GameplayStatics.SetGamePaused` true))

(event `EnhancedInput|/Game/Player/Input/IA_PauseGame`
  (params (ActionValue :type Boolean) (ElapsedSeconds :type "Float (double-precision)") (TriggeredSeconds :type "Float (double-precision)") (InputAction :type "InputAction Object Reference" :default "/Game/Player/Input/IA_PauseGame.IA_PauseGame"))
  (:`Started`
    (if (not (`self.IsGameEnded`))
      (if (not (`self.IsPauseMesuOpened`))
        (`self.PauseGame`)
        (else
          (set `self.IsPauseMesuOpened` false)
          (`Widget.RemoveFromParent` (`self.PauseMenu`))
          (`GameplayStatics.SetGamePaused` false)
          (`WidgetBlueprintLibrary.SetInputMode_GameOnly` (`GameplayStatics.GetPlayerController` 0))
          (set `PlayerController.bShowMouseCursor` false (`GameplayStatics.GetPlayerController` 0)))))))

(event `StageCleared`
  (bind _returnvalue (`GameplayStatics.GetCurrentLevelName` true))
  (set `self.ClearedStage` (`KismetStringLibrary.Conv_StringToInt` _returnvalue))
  (`KismetSystemLibrary.PrintString` (`KismetStringLibrary.Concat_StrStr` _returnvalue " 클리어") true true (struct :`G` 0.66 :`B` 1.0 :`A` 1.0) 20.0)
  (bind _beststage (message `/Game/Player/Blueprints/Interfaces/BPI_GameInstance.GetBestStage` (`GameplayStatics.GetGameInstance`)))
  (if (<= _beststage (`self.ClearedStage`))
    (message `/Game/Player/Blueprints/Interfaces/BPI_GameInstance.SetBestStage` (`GameplayStatics.GetGameInstance`) (`self.ClearedStage`))))

(event `BestStage`)

(event `StageFailed`)

(fn `UserConstructionScript`)