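; BP_Deer is an AI deer character that dies when it overlaps a BP_Arrow.
; Death hides the incoming arrow, shows a right-side or default embedded arrow depending on the BodyRight overlap, plays a death montage, then hides the deer after a delay.
; On BeginPlay it stores a BP_AIPoints actor as its patrol reference.
; While alive, Tick randomizes walk speed once each time movement stops.
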(event `Death`
  (set `self.IsDead` true)
  (`SceneComponent.SetVisibility` (`Actor.RootComponent` (`self.ArrowInstance`)) false true)
  (if (`self.RightHit`)
    (`SceneComponent.SetVisibility` (`self.PlayerArrowRight`) true true)
    (else
      (`SceneComponent.SetVisibility` (`self.PlayerArrow`) true true)))
  (`MovementComponent.StopMovementImmediately` (`self.CharacterMovement`))
  (`|PlayMontage` (`self.Mesh`) "/Game/AnimalVarietyPack/DeerStagAndDoe/Animations/AM_Deer_HitDeath.AM_Deer_HitDeath"
    (:`then`
      (`KismetSystemLibrary.Delay` 3.5)
      (for _array_element (`|MakeArray` (`self.PlayerArrowRight`) (`self.PlayerArrow`))
        (`SceneComponent.SetVisibility` _array_element false false)
        (`SceneComponent.SetVisibility` (`self.Mesh`) false false)))))

(event `self.ReceiveActorBeginOverlap`
  (params (OtherActor :type "Actor Object Reference"))
  (bind _asbp_arrow (cast `/Game/Player/Blueprints/BP_Arrow` OtherActor))
  (set `self.ArrowInstance` _asbp_arrow)
  (`self.Death`))

(event `self.BodyRight.OnComponentBeginOverlap`
  (params (OverlappedComponent :type "PrimitiveComponent Object Reference") (OtherActor :type "Actor Object Reference") (OtherComp :type "PrimitiveComponent Object Reference") (OtherBodyIndex :type Integer) (bFromSweep :type Boolean) (SweepResult :type "HitResult Structure (by ref)"))
  (cast `/Game/Player/Blueprints/BP_Arrow` OtherActor)
  (set `self.RightHit` true))

(event `self.ReceiveBeginPlay`
  (`SceneComponent.SetVisibility` (`self.PlayerArrow`) false false)
  (`SceneComponent.SetVisibility` (`self.PlayerArrowRight`) false false)
  (bind _outactors (`GameplayStatics.GetAllActorsOfClass` "/Game/Player/AI/BP_AIPoints.BP_AIPoints_C"))
  (for _array_element _outactors
    (bind _asbp_aipoints (cast `/Game/Player/AI/BP_AIPoints` _array_element))
    (set `self.PatrolPoints` _asbp_aipoints)))

(event `self.ReceiveTick`
  (params (DeltaSeconds :type "Float (single-precision)"))
  (`|ExecutionSequence`
    (:`then_1`
      (if (`self.IsDead`)
        _
        (elif (> (`KismetMathLibrary.VSize` (`MovementComponent.Velocity` (`self.CharacterMovement`))) 0.0)
          (if (`self.ChangeSpeed`)
            (set `self.ChangeSpeed` false))
          (elif (not (`self.ChangeSpeed`))
            (set `CharacterMovementComponent.MaxWalkSpeed` (`KismetMathLibrary.RandomFloatInRange` 200.0 600.0) (`self.CharacterMovement`))
            (set `self.ChangeSpeed` true)))))))

(fn `UserConstructionScript`)