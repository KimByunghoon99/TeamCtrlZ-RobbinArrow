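; Deer AI character that patrol-point actors feed and that dies when hit by an arrow.
; Body, front and head overlaps flag the hit side, so death hides the arrow and reveals the matching pre-attached arrow mesh.
; Death plays a montage, records the transform in GM_RobbinArrow, then destroys the deer after a delay.
; Tick re-randomizes walk speed whenever a living deer comes to a stop, while BeginPlay caches a BP_AIPointsDeer.
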(event `Death`
  (set `self.IsDead` true)
  (`SceneComponent.SetVisibility` (`Actor.RootComponent` (`self.ArrowInstance`)) false true)
  (if (`self.RightHit`)
    (`SceneComponent.SetVisibility` (`self.PlayerArrowRight`) true true)
    (elif (`self.FrontHit`)
      (`SceneComponent.SetVisibility` (`self.PlayerArrowFront`) true true)
      (else
        (`SceneComponent.SetVisibility` (`self.PlayerArrow`) true true))))
  (`MovementComponent.StopMovementImmediately` (`self.CharacterMovement`))
  (`PrimitiveComponent.SetCollisionEnabled` (`self.Mesh`) "NoCollision")
  (`|PlayMontage` (`self.Mesh`) "/Game/AnimalVarietyPack/DeerStagAndDoe/Animations/AM_Deer_HitDeath.AM_Deer_HitDeath"
    (:`then`
      (bind _asgm_robbin_arrow (cast `/Game/Player/Blueprints/GM_RobbinArrow` (`GameplayStatics.GetGameMode`)))
      (`KismetArrayLibrary.Array_Add` (`/Game/Player/Blueprints/GM_RobbinArrow.DeerTransformArray` _asgm_robbin_arrow) (`self.GetTransform`))
      (`KismetSystemLibrary.Delay` 3.5)
      (`self.K2_DestroyActor`))))

(event `self.BodyRight.OnComponentBeginOverlap`
  (params (OverlappedComponent :type "PrimitiveComponent Object Reference") (OtherActor :type "Actor Object Reference") (OtherComp :type "PrimitiveComponent Object Reference") (OtherBodyIndex :type Integer) (bFromSweep :type Boolean) (SweepResult :type "HitResult Structure (by ref)"))
  (cast `/Game/Player/Blueprints/BP_Arrow` OtherActor)
  (set `self.RightHit` true))

(event `self.ReceiveBeginPlay`
  (`SceneComponent.SetVisibility` (`self.PlayerArrowFront`) false false)
  (`SceneComponent.SetVisibility` (`self.PlayerArrow`) false false)
  (`SceneComponent.SetVisibility` (`self.PlayerArrowRight`) false false)
  (bind _outactors (`GameplayStatics.GetAllActorsOfClass` "/Game/Player/AI/Deer/BP_AIPointsDeer.BP_AIPointsDeer_C"))
  (for _array_element _outactors
    (bind _asbp_aipoints (cast `/Game/Player/AI/Deer/BP_AIPointsDeer` _array_element))
    (set `self.PatrolPoints` _asbp_aipoints)))

(event `self.Front.OnComponentBeginOverlap`
  (params (OverlappedComponent :type "PrimitiveComponent Object Reference") (OtherActor :type "Actor Object Reference") (OtherComp :type "PrimitiveComponent Object Reference") (OtherBodyIndex :type Integer) (bFromSweep :type Boolean) (SweepResult :type "HitResult Structure (by ref)"))
  (cast `/Game/Player/Blueprints/BP_Arrow` (stale `self.Head.OnComponentBeginOverlap` OtherActor) :!label _label)
  (set `self.FrontHit` true))

(event `self.ReceiveTick`
  (params (DeltaSeconds :type "Float (single-precision)"))
  (`|ExecutionSequence`
    (:`then_1`
      (if (`self.IsDead`)
        _
        (elif (> (`KismetMathLibrary.VSize` (`MovementComponent.Velocity` (`self.CharacterMovement`))) 0.0)
          (if (`self.ChangeSpeed`)
            (set `self.ChangeSpeed` false))
          (elif (not (`self.ChangeSpeed`))
            (set `CharacterMovementComponent.MaxWalkSpeed` (`KismetMathLibrary.RandomFloatInRange` 200.0 600.0) (`self.CharacterMovement`))
            (set `self.ChangeSpeed` true)))))))

(event `self.Head.OnComponentBeginOverlap`
  (params (OverlappedComponent :type "PrimitiveComponent Object Reference") (OtherActor :type "Actor Object Reference") (OtherComp :type "PrimitiveComponent Object Reference") (OtherBodyIndex :type Integer) (bFromSweep :type Boolean) (SweepResult :type "HitResult Structure (by ref)"))
  (goto _label))

(event `self.ReceiveActorBeginOverlap`
  (params (OtherActor :type "Actor Object Reference"))
  (if (!= OtherActor self)
    (bind _asbp_arrow (cast `/Game/Player/Blueprints/BP_Arrow` OtherActor))
    (set `self.ArrowInstance` _asbp_arrow)
    (`self.Death`)))

(fn `UserConstructionScript`)