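; BP_Kraken is a kraken that surfaces to attack after a random delay at spawn.
; Attack plays a pre-attack montage with sounds, then a timeline lifts it up and along negative Y by a random distance before setting AttackOn.
; Dive, not called in this graph, reverses that path on a second timeline at half custom time dilation, then schedules the next Attack.
; AttackOn is never cleared after BeginPlay here.
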(event `self.ReceiveBeginPlay`
  (set `self.AttackOn` false)
  (`KismetSystemLibrary.Delay` (`KismetMathLibrary.RandomFloatInRange` 1.0 3.0))
  (`self.Attack`))

(event `Attack`
  (bind (_startloction_x _startloction_y _startloction_z) (`KismetMathLibrary.BreakVector` (`self.StartLoction`)))
  (`GameplayStatics.PlaySoundAtLocation` "/Game/Player/Sound/Cue_Kraken_Growl.Cue_Kraken_Growl" (`self.K2_GetActorLocation`) (struct) 1.0 1.0 0.0 null null null null)
  (`|PlayMontage` (`self.Mesh`) "/Game/Player/Animations/AM_Kraken_PreAttack.AM_Kraken_PreAttack"
    (:`then`
      (`KismetSystemLibrary.Delay` 0.2)
      (`GameplayStatics.PlaySoundAtLocation` "/Game/Player/Sound/Cue_WaterCasting.Cue_WaterCasting" (`self.K2_GetActorLocation`) (struct) 0.5 1.0 0.0 null null null null))
    (:`OnCompleted`
      (set `self.StartLoction` (`self.K2_GetActorLocation`))
      (set `self.RandomFloat` (`KismetMathLibrary.RandomFloatInRange` 1400.0 1800.0))
      (`GameplayStatics.PlaySoundAtLocation` "/Game/Player/Sound/Cue_Kraken_Attack.Cue_Kraken_Attack" (`self.K2_GetActorLocation`) (struct) 0.85 1.0 0.0 null null null null)
      (`|ExecutionSequence`
        (:`then_0`
          (`KismetSystemLibrary.Delay` 0.2)
          (`GameplayStatics.PlaySoundAtLocation` "/Game/Player/Sound/Cue_WaterSplash.Cue_WaterSplash" (`self.K2_GetActorLocation`) (struct) 0.7 1.0 0.0 null null null null))
        (:`then_1`
          (bind (_direction _newtrack_0) (`Timeline|MoveUP` :!via `PlayFromStart`)
            (:`Update`
              (`self.K2_SetActorLocation` (`KismetMathLibrary.MakeVector` _startloction_x (`KismetMathLibrary.Lerp` _startloction_y (- _startloction_y (`self.RandomFloat`)) _newtrack_0) (`KismetMathLibrary.Lerp` _startloction_z (+ _startloction_z 800.0) _newtrack_0))))
            (:`Finished`
              (`KismetSystemLibrary.Delay` (`KismetMathLibrary.RandomFloatInRange` 0.5 2.0))
              (set `self.AttackOn` true))))))))

(event `Dive`
  (bind (_startloction_x _startloction_y _startloction_z) (`KismetMathLibrary.BreakVector` (`self.StartLoction`)))
  (set `self.CustomTimeDilation` 0.5)
  (`|ExecutionSequence`
    (:`then_0`
      (bind (_direction _newtrack_0) (`Timeline|Timeline` :!via `ReverseFromEnd`)
        (:`Update`
          (`self.K2_SetActorLocation` (`KismetMathLibrary.MakeVector` _startloction_x (`KismetMathLibrary.Lerp` _startloction_y (- _startloction_y (`self.RandomFloat`)) _newtrack_0) (`KismetMathLibrary.Lerp` _startloction_z (+ _startloction_z 800.0) _newtrack_0))))
        (:`Finished`
          (set `self.CustomTimeDilation` 1.0)
          (`KismetSystemLibrary.Delay` (`KismetMathLibrary.RandomFloatInRange` 3.0 6.0))
          (`self.Attack`))))
    (:`then_1`
      (`KismetSystemLibrary.Delay` 0.8)
      (`GameplayStatics.PlaySoundAtLocation` "/Game/Player/Sound/Cue_WaterSplash.Cue_WaterSplash" (`self.K2_GetActorLocation`) (struct) 0.5 0.8 0.0 null null null null))))

(fn `UserConstructionScript`)